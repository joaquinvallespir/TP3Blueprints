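; BP_Enemyexplosive is a twin-stick shooter enemy that chases the player and self-destructs on arrival.
; Pawn sensing starts an AI move toward the seen TwinStickPawn, and success destroys the enemy with an explosion effect but applies no damage.
; Capsule overlaps recognize projectiles by display-name substring, destroy them and decrement Health, removing the enemy without an explosion at zero.
; GameMode casts drive nothing, as the EnemyAlive increment never runs.
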(event OnSeePawn(PawnSensing)
  (params (Pawn :type Pawn%20Object%20Reference))
  (bind _astwin_stick_pawn (Utilities|Casting|CastToTwinStickPawn Pawn))
  (AI|AIMoveTo self "0, 0, 0" _astwin_stick_pawn 5.0 false
    (:OnSuccess
      (Actor|DestroyActor)
      (Effects|SpawnEmitteratLocation "/Game/StarterContent/Particles/P_Explosion.P_Explosion" (Transformation|GetActorLocation)))))

(event OnComponentBeginOverlap(CapsuleComponent)
  (params (OverlappedComponent :type Primitive%20Component%20Object%20Reference) (OtherActor :type Actor%20Object%20Reference) (OtherComp :type Primitive%20Component%20Object%20Reference) (OtherBodyIndex :type Integer) (bFromSweep :type Boolean) (SweepResult :type Hit%20Result%20Structure%20%28by%20ref%29))
  (if (Utilities|String|Contains (Utilities|GetDisplayName OtherActor) "TwinStickProjectile")
    (Actor|DestroyActor OtherActor)
    (bind _result (Math|Integer|DecrementInt (Variables|Default|GetHealth))
      (:%20%20
        (Variables|Default|SetHealth _result)
        (if (== (Variables|Default|GetHealth) 0)
          (Utilities|Casting|CastToTwinStickGameMode (Game|GetGameMode))
          (Class|Pawn|DetachfromControllerPendingDestroy)
          (Actor|DestroyActor))))))

(fn ConstructionScript
  (Utilities|Casting|CastToTwinStickGameMode (Game|GetGameMode)))